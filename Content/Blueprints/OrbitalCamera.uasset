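; Orbital camera Blueprint that swings its CameraArm left or right while the matching rotation flag is set.
; BeginPlay clears both flags, and Tick checks each independently to call RotateL or RotateR; nothing in this file sets them true.
; Each call combines the arm's world rotation with a fixed step, ignoring the passed DeltaSeconds, so orbit speed depends on frame rate.
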(event EventBeginPlay
  (Variables|Default|SetRotateLeft false)
  (Variables|Default|SetRotateRight false))

(event Collision|EventActorBeginOverlap
  (params (OtherActor :type Actor%20Object%20Reference)))

(event EventTick
  (params (DeltaSeconds :type Float%20%28single-precision%29))
  (Utilities|FlowControl|Sequence
    (:then_0
      (if (Variables|Default|GetRotateLeft)
        (CallFunction|RotateL DeltaSeconds)))
    (:then_1
      (if (Variables|Default|GetRotateRight)
        (CallFunction|RotateR DeltaSeconds)))))

(fn ConstructionScript)

(fn RotateL
  (params (DeltaSeconds :type Float%20%28double-precision%29))
  (bind _cameraarm (Variables|Default|GetCameraArm))
  (if true
    (Transformation|SetWorldRotation _cameraarm (Math|Rotator|CombineRotators (Transformation|GetWorldRotation _cameraarm) "0.000000,-3.000000,0.000000") false false)))

(fn RotateR
  (params (DeltaSeconds :type Float%20%28double-precision%29))
  (bind _cameraarm (Variables|Default|GetCameraArm))
  (if true
    (Transformation|SetWorldRotation _cameraarm (Math|Rotator|CombineRotators (Transformation|GetWorldRotation _cameraarm) "0.000000,3.000000,0.000000") false false)))