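; Player character that steps sideways with MoveLeft and MoveRight inputs, relative to the current camera side.
; BeginPlay caches the VP-GameController, whose CameraActor string (N, S, E, W) selects the axis and sign of each fixed-step Teleport, which also zeroes rotation.
; The E and W branches compute the new Y from the current X location.
; Both inputs also print CameraActor, and the Orbit-based CanMove logic is unconnected.
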(event EventBeginPlay
  (bind _asvp_game_controller (Utilities|Casting|CastToVP-GameController (Pawn|GetController)))
  (Variables|Default|SetGame-Controller _asvp_game_controller))

(event Input|ActionEvents|InputActionMoveRight
  (params (Key :type Key%20Structure :default "None"))
  (bind _returnvalue (Transformation|GetActorLocation))
  (bind _game_controller (Variables|Default|GetGame-Controller))
  (bind (_x _y _z) (Class|KismetMathLibrary|BreakVector3f _returnvalue))
  (bind _cameraactor (Variables|/Game/Blueprints/VP-GameController.VP-GameController_C|GetCameraActor _game_controller))
  (:Pressed
    (if true
      (if (Utilities|Enum|Equal(Enum) _cameraactor "N")
        (bind _output_get (Variables|Default|SetLocation (Math|Vector|MakeVector (+ _x -1e+02) _y _z)))
        (Utilities|FlowControl|Delay 0.0)
        (Transformation|Teleport _output_get "0, 0, 0")
        (elif (Utilities|Enum|Equal(Enum) _cameraactor "S")
          (bind _output_get_2 (Variables|Default|SetLocation (Math|Vector|MakeVector (+ _x 1e+02) _y _z)))
          (Utilities|FlowControl|Delay 0.0)
          (Transformation|Teleport _output_get_2 "0, 0, 0")
          (elif (Utilities|Enum|Equal(Enum) _cameraactor "E")
            (bind _output_get_3 (Variables|Default|SetLocation (Math|Vector|MakeVector _x (+ _x 5e+01) _z)))
            (Utilities|FlowControl|Delay 0.0)
            (Transformation|Teleport _output_get_3 "0, 0, 0")
            (elif (Utilities|Enum|Equal(Enum) _cameraactor "W")
              (bind _output_get_4 (Variables|Default|SetLocation (Math|Vector|MakeVector _x (+ _x -5e+01) _z)))
              (Utilities|FlowControl|Delay 0.0)
              (Transformation|Teleport _output_get_4 "0, 0, 0"))))))))

(event Input|ActionEvents|InputActionMoveRight
  (params (Key :type Key%20Structure :default "None"))
  (:Pressed
    (Development|PrintString (Variables|/Game/Blueprints/VP-GameController.VP-GameController_C|GetCameraActor (Variables|Default|GetGame-Controller)))))

(event Input|ActionEvents|InputActionMoveLeft
  (params (Key :type Key%20Structure :default "None"))
  (bind _returnvalue (Transformation|GetActorLocation))
  (bind _game_controller (Variables|Default|GetGame-Controller))
  (bind (_x _y _z) (Class|KismetMathLibrary|BreakVector3f _returnvalue))
  (bind _cameraactor (Variables|/Game/Blueprints/VP-GameController.VP-GameController_C|GetCameraActor _game_controller))
  (:Pressed
    (if true
      (if (Utilities|Enum|Equal(Enum) _cameraactor "N")
        (bind _output_get (Variables|Default|SetLocation (Math|Vector|MakeVector (+ _x 1e+02) _y _z)))
        (Utilities|FlowControl|Delay 0.0)
        (Transformation|Teleport _output_get "0, 0, 0")
        (elif (Utilities|Enum|Equal(Enum) _cameraactor "S")
          (bind _output_get_2 (Variables|Default|SetLocation (Math|Vector|MakeVector (+ _x -1e+02) _y _z)))
          (Utilities|FlowControl|Delay 0.0)
          (Transformation|Teleport _output_get_2 "0, 0, 0")
          (elif (Utilities|Enum|Equal(Enum) _cameraactor "E")
            (bind _output_get_3 (Variables|Default|SetLocation (Math|Vector|MakeVector _x (+ _x -5e+01) _z)))
            (Utilities|FlowControl|Delay 0.0)
            (Transformation|Teleport _output_get_3 "0, 0, 0")
            (elif (Utilities|Enum|Equal(Enum) _cameraactor "W")
              (bind _output_get_4 (Variables|Default|SetLocation (Math|Vector|MakeVector _x (+ _x 5e+01) _z)))
              (Utilities|FlowControl|Delay 0.0)
              (Transformation|Teleport _output_get_4 "0, 0, 0"))))))))

(event Input|ActionEvents|InputActionMoveLeft
  (params (Key :type Key%20Structure :default "None"))
  (:Pressed
    (Development|PrintString (Variables|/Game/Blueprints/VP-GameController.VP-GameController_C|GetCameraActor (Variables|Default|GetGame-Controller)))))

(fn ConstructionScript)