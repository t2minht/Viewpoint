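; RoomBox is a room trigger volume that switches the player's view to that room's directional cameras.
; On any box overlap it casts its four child-actor cameras (N, S, E, W) and stores them on the VPGameController as the current camera set.
; It then calls SetViewTargetWithBlend on the controller to the camera matching its CameraActor direction value, keeping the same facing between rooms.
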(event OnComponentBeginOverlap(Box)
  (params (OverlappedComponent :type Primitive%20Component%20Object%20Reference) (OtherActor :type Actor%20Object%20Reference) (OtherComp :type Primitive%20Component%20Object%20Reference) (OtherBodyIndex :type Integer) (bFromSweep :type Boolean) (SweepResult :type Hit%20Result%20Structure%20%28by%20ref%29))
  (bind _returnvalue (Actor|GetActorOfClass "/Game/Blueprints/VP-GameController.VP-GameController_C"))
  (bind _ascamera_actor_e (Utilities|Casting|CastToCameraActorE (Variables|/Script/Engine.ChildActorComponent|GetChildActor (Variables|Default|GetCameraActorE))))
  (bind _output_get (Variables|/Game/Blueprints/VP-GameController.VP-GameController_C|SetECam _returnvalue _ascamera_actor_e))
  (bind _ascamera_actor_w (Utilities|Casting|CastToCameraActorW (Variables|/Script/Engine.ChildActorComponent|GetChildActor (Variables|Default|GetCameraActorW))))
  (bind _output_get_2 (Variables|/Game/Blueprints/VP-GameController.VP-GameController_C|SetWCam _returnvalue _ascamera_actor_w))
  (bind _ascamera_actor_n (Utilities|Casting|CastToCameraActorN (Variables|/Script/Engine.ChildActorComponent|GetChildActor (Variables|Default|GetCameraActorN))))
  (bind _output_get_3 (Variables|/Game/Blueprints/VP-GameController.VP-GameController_C|SetNCam _returnvalue _ascamera_actor_n))
  (bind _ascamera_actor_s (Utilities|Casting|CastToCameraActorS (Variables|/Script/Engine.ChildActorComponent|GetChildActor (Variables|Default|GetCameraActorS))))
  (bind _output_get_4 (Variables|/Game/Blueprints/VP-GameController.VP-GameController_C|SetSCam _returnvalue _ascamera_actor_s))
  (if (Utilities|Enum|Equal(Enum) (Variables|/Game/Blueprints/VP-GameController.VP-GameController_C|GetCameraActor _returnvalue) "N")
    (Game|Player|SetViewTargetwithBlend _returnvalue _output_get_3 0.0 "VTBlend_Linear" 0.0 false)
    (elif (Utilities|Enum|Equal(Enum) (Variables|/Game/Blueprints/VP-GameController.VP-GameController_C|GetCameraActor _returnvalue) "S")
      (Game|Player|SetViewTargetwithBlend _returnvalue _output_get_4 0.0 "VTBlend_Linear" 0.0 false)
      (elif (Utilities|Enum|Equal(Enum) (Variables|/Game/Blueprints/VP-GameController.VP-GameController_C|GetCameraActor _returnvalue) "E")
        (Game|Player|SetViewTargetwithBlend _returnvalue _output_get 0.0 "VTBlend_Linear" 0.0 false)
        (elif (Utilities|Enum|Equal(Enum) (Variables|/Game/Blueprints/VP-GameController.VP-GameController_C|GetCameraActor _returnvalue) "W")
          (Game|Player|SetViewTargetwithBlend _returnvalue _output_get_2 0.0 "VTBlend_Linear" 0.0 false))))))

(event EventBeginPlay)

(event Collision|EventActorBeginOverlap
  (params (OtherActor :type Actor%20Object%20Reference)))

(event EventTick
  (params (DeltaSeconds :type Float%20%28single-precision%29)))

(fn ConstructionScript)